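; BP_Paddle is a player-controlled paddle that moves sideways with swept movement through Enhanced Input.
; It registers IMC_InGame on BeginPlay, and IA_Action calls Action on the BP_GameManager found in the level.
; GetTopNormal fakes a curved top by rolling upward hit normals in proportion to Y offset from center, up to MaxTiltNormalDeg.
; Every Tick, it draws debug arrows of these tilted normals across the top surface.
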(event Input|EnhancedActionEvents|EnhancedInputActionIA_Move
  (params (ActionValue :type Float%20%28double-precision%29) (ElapsedSeconds :type Float%20%28double-precision%29) (TriggeredSeconds :type Float%20%28double-precision%29) (InputAction :type Input%20Action%20Object%20Reference :default "/Game/InputAction/IA_Move.IA_Move"))
  (Transformation|SetActorLocation (+ (* (* (* (Class|KismetMathLibrary|VectorRight) ActionValue) (Variables|Default|GetSpeed)) (Utilities|Time|GetWorldDeltaSeconds)) (Transformation|GetActorLocation)) true false))

(event Input|EnhancedActionEvents|EnhancedInputActionIA_Action
  (params (ActionValue :type Boolean) (ElapsedSeconds :type Float%20%28double-precision%29) (TriggeredSeconds :type Float%20%28double-precision%29) (InputAction :type Input%20Action%20Object%20Reference :default "/Game/InputAction/IA_Action.IA_Action"))
  (:Started
    (Default|Action (Variables|Default|GetGameManager))))

(event EventBeginPlay
  (Input|AddMappingContext (PlayerController|LocalPlayerSubsystems|GetEnhancedInputLocalPlayerSubsystem (Game|GetPlayerController 0)) "/Game/InputAction/IMC_InGame.IMC_InGame" 0 "(bIgnoreAllPressedKeysUntilRelease=True,bForceImmediately=False,bNotifyUserSettings=False)")
  (bind _returnvalue (Actor|GetActorOfClass "/Game/BluePrint/BP_GameManager.BP_GameManager_C"))
  (Variables|Default|SetGameManager _returnvalue))

(event Collision|EventActorBeginOverlap
  (params (OtherActor :type Actor%20Object%20Reference)))

(event EventTick
  (params (DeltaSeconds :type Float%20%28single-precision%29))
  (CallFunction|DrawDebugTopSurfaceNormals))

(fn ConstructionScript)

(fn GetTopNormal
  (params (HitLodation :type Vector) (Normal :type Vector))
  (bind (_origin _boxextent) (Collision|GetActorBounds false false))
  (if (Class|KismetMathLibrary|NotEqualExactlyVectorVector Normal (Math|Vector|VectorUp))
    (return false Normal)
    (else
      (return true (Math|Vector|RotateVector Normal (Math|Rotator|MakeRotator (* (/ (- (.Y (Math|Vector|BreakVector HitLodation)) (.y _origin)) (.y _boxextent)) (Variables|Default|GetMaxTiltNormalDeg)) 0.0 0.0))))))

(fn DrawDebugArrow
  (params (Origin :type Vector) (Direction :type Vector))
  (LocalVariables|SetL_ShapeDirection (* (Math|Vector|Normalize Direction) (LocalVariables|GetL_Length)))
  (Rendering|Debug|DrawDebugArrow Origin (+ (LocalVariables|GetL_ShapeDirection) Origin) 1e+02 "(R=0.042698,G=0.000000,B=1.000000,A=1.000000)" 0.0 1e+01))

(fn DrawDebugTopSurfaceNormals
  (bind (_origin _boxextent) (Collision|GetActorBounds false false))
  (for _index (range (* (LocalVariables|GetL_DrawNumHalf) -1) (LocalVariables|GetL_DrawNumHalf))
    (bind _outnormal (CallFunction|GetTopNormal (+ (Math|Vector|MakeVector 0.0 (* _index (/ (.y _boxextent) (LocalVariables|GetL_DrawNumHalf))) (.z _boxextent)) _origin) (Math|Vector|VectorUp)))
    (CallFunction|DrawDebugArrow (+ (Math|Vector|MakeVector 0.0 (* _index (/ (.y _boxextent) (LocalVariables|GetL_DrawNumHalf))) (.z _boxextent)) _origin) _outnormal)))